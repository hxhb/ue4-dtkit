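; A game mode that drives a file download test through an on-screen BP_DownloadProxy widget.
; On BeginPlay it shows the cursor and binds the widget's start, pause, resume, cancel and reset events to a DownloadProxy object created per URL.
; Proxy delegates print pause, resume and completion, with a hard-coded hash check on success.
; Tick prints progress and speed once progress is nonzero.
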(event Custom|Complete
  (params (Proxy :type Download%20Proxy%20Object%20Reference) (bSuccess :type Boolean))
  (Development|PrintString (Utilities|String|Append "Download Complete: " (Utilities|String|ToString(Boolean) bSuccess)))
  (if bSuccess
    (Development|PrintString (Utilities|String|Append "Hash Check is " (Utilities|String|ToString(Boolean) (Class|DownloadProxy|HashCheck Proxy "CDBCA2A78AC94860FCDC6C24414CB9F1"))))))

(event Custom|Pause
  (params (Proxy :type Download%20Proxy%20Object%20Reference))
  (Development|PrintString (Utilities|String|Append (Utilities|GetDisplayName Proxy) "  Download Mission is pause.")))

(event Custom|Resume
  (params (Proxy :type Download%20Proxy%20Object%20Reference))
  (Development|PrintString (Utilities|String|Append (Utilities|GetDisplayName Proxy) " Download Mission is RESUME.")))

(event Custom|OnStartDownload
  (params (URL :type String))
  (bind _returnvalue (Game|ConstructObjectfromClass "/Script/GameUpdater.DownloadProxy" self))
  (EventDispatchers|BindEventtoOnDownloadCompleteDyMulitDlg _returnvalue (delegate Custom|Complete))
  (Class|DownloadProxy|RequestDownload _returnvalue URL)
  (bind _output_get (Variables|Default|SetDownloadObj _returnvalue))
  (EventDispatchers|BindEventtoOnDownloadPausedDyMulitDlg _output_get (delegate Custom|Pause))
  (EventDispatchers|BindEventtoOnDownloadResumedDyMulitDlg _output_get (delegate Custom|Resume)))

(event Custom|UIPause
  (Class|DownloadProxy|Pause (Variables|Default|GetDownloadObj)))

(event Custom|UIResume
  (Class|DownloadProxy|Resume (Variables|Default|GetDownloadObj)))

(event Custom|UICancel
  (Class|DownloadProxy|Cancel (Variables|Default|GetDownloadObj)))

(event Custom|UIReset
  (Class|DownloadProxy|Reset (Variables|Default|GetDownloadObj)))

(event EventBeginPlay
  (bind _returnvalue (Game|GetPlayerController 0))
  (Variables|/Script/Engine.PlayerController|SetbShowMouseCursor _returnvalue true)
  (bind _returnvalue_2 (UserInterface|CreateWidget "/GameUpdater/BP_DownloadProxy.BP_DownloadProxy_C" _returnvalue))
  (bind _output_get (Variables|Default|SetDownloadUI _returnvalue_2))
  (UserInterface|Viewport|AddtoViewport _output_get 0)
  (EventDispatchers|BindEventtoOnStartDownload _output_get (delegate Custom|OnStartDownload))
  (EventDispatchers|BindEventtoOnPause _output_get (delegate Custom|UIPause))
  (EventDispatchers|BindEventtoOnResume (Variables|Default|GetDownloadUI) (delegate Custom|UIResume))
  (EventDispatchers|BindEventtoOnCancel (Variables|Default|GetDownloadUI) (delegate Custom|UICancel))
  (EventDispatchers|BindEventtoOnReset (Variables|Default|GetDownloadUI) (delegate Custom|UIReset)))

(event EventTick
  (params (DeltaSeconds :type Float%20%28single-precision%29))
  (bind _downloadobj (Variables|Default|GetDownloadObj))
  (bind _returnvalue (Class|DownloadProxy|GetDownloadProgress _downloadobj))
  (if (Utilities|IsValid _downloadobj)
    (if (!= _returnvalue 0.0)
      (Development|PrintString (Utilities|String|Append "Progress:" (Utilities|String|ToString(Float) _returnvalue) " Speed:" (Utilities|String|ToString(Float) (Class|DownloadProxy|GetDownloadSpeedKbs _downloadobj)) "kb/s")))))

(fn ConstructionScript)